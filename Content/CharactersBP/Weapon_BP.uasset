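; Weapon Blueprint that handles firing, ammo and timed reloading for a gun.
; Fire spawns a Bullet_BP at the skeletal mesh's Muzzle socket, passes it the damage range, plays the shot sound, spends a round and emits noise events.
; Firing on an empty magazine falls into the same path as Reload, which plays an attenuated sound, waits out a delay guarded by a Reloading flag, then refills ammo to maximum.
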(event Custom|Fire
  (bind _returnvalue (Game|GetInstigator))
  (bind _returnvalue_2 (Transformation|GetActorLocation))
  (bind _skeletalmesh (Variables|Default|GetSkeletalMesh))
  (bind _returnvalue_3 (Transformation|GetSocketTransform _skeletalmesh "Muzzle" "RTS_World"))
  (if (and (>= (Variables|Default|GetAmmo) 1) (not (Variables|Default|GetReloading)))
    (bind _returnvalue_4 (Game|SpawnActorfromClass "/Game/CharactersBP/Bullet_BP.Bullet_BP_C" (Math|Transform|MakeTransform (.location _returnvalue_3) (.rotation _returnvalue_3) "0.100000,0.100000,0.100000") "AdjustIfPossibleButAlwaysSpawn" 0 0))
    (if (Utilities|IsValid _returnvalue_4)
      (Variables|/Game/CharactersBP/Bullet_BP.Bullet_BP_C|SetMaxDamage _returnvalue_4 (Variables|Default|GetMaxBulletDamage))
      (Variables|/Game/CharactersBP/Bullet_BP.Bullet_BP_C|SetMinDamage _returnvalue_4 (Variables|Default|GetMinBulletDamage)))
    (Audio|SpawnSoundatLocation (Variables|Default|GetFiringSound) (Transformation|GetActorLocation) "0, 0, 0" 0.5 1.0 0.0 "/Game/CharactersBP/GunSoundAttenuation_BP.GunSoundAttenuation_BP" 0)
    (Math|Integer|DecrementInt (Variables|Default|GetAmmo)
      (:%20%20
        (Class|AISenseHearing|ReportNoiseEvent _returnvalue_2 1.0 _returnvalue 0.0 "None")
        (Class|Actor|MakeNoise self 1.0 _returnvalue _returnvalue_2 0.0 "None")))
    (elif (not (Variables|Default|GetReloading))
      (Variables|Default|SetReloading true)
      (Audio|SpawnSoundatLocation "/Game/Assets/Audio/Loading.Loading" (Transformation|GetActorLocation) "0, 0, 0" 0.5 0.5 0.0 "/Game/CharactersBP/ReloadAndWalkSoundAttenuation.ReloadAndWalkSoundAttenuation" 0)
      (Utilities|FlowControl|Delay (Variables|Default|GetReloadingTime))
      (Variables|Default|SetAmmo (Variables|Default|GetMaxAmmo))
      (Variables|Default|SetReloading false))))

(event Custom|Reload
  (if (not (Variables|Default|GetReloading))
    (Variables|Default|SetReloading true)
    (Audio|SpawnSoundatLocation "/Game/Assets/Audio/Loading.Loading" (Transformation|GetActorLocation) "0, 0, 0" 0.5 0.5 0.0 "/Game/CharactersBP/ReloadAndWalkSoundAttenuation.ReloadAndWalkSoundAttenuation" 0)
    (Utilities|FlowControl|Delay (Variables|Default|GetReloadingTime))
    (Variables|Default|SetAmmo (Variables|Default|GetMaxAmmo))
    (Variables|Default|SetReloading false)))

(event EventBeginPlay)

(event Collision|EventActorBeginOverlap
  (params (OtherActor :type Actor%20Object%20Reference)))

(event EventTick
  (params (DeltaSeconds :type Float%20%28single-precision%29)))

(fn ConstructionScript)